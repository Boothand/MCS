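; MCS game state base that controls global time dilation.
; Increase, decrease and reset events all feed one setter, which stores the current dilation and applies it globally without clamping.
; A GetGameMode helper returns the game mode cast to MCSGameModeDuel and reports invalid cast info when the cast fails.
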(event Custom|OnSetTimeDilation
  (params (Dilation%20Amount :type Float%20%28single-precision%29))
  ;[1 1 1] Global time dilation
  (bind _output_get (Variables|TimeFX|SetCurrentTimeDilation Dilation%20Amount))
  (Utilities|Time|SetGlobalTimeDilation _output_get))

(event Custom|OnIncreaseTime
  ;[1 1 1] Global time dilation
  (CallFunction|OnSetTimeDilation (+ (Variables|TimeFX|GetCurrentTimeDilation) (Variables|TimeFX|GetTimeDilationStep))))

(event Custom|OnDecreaseTime
  ;[1 1 1] Global time dilation
  (CallFunction|OnSetTimeDilation (- (Variables|TimeFX|GetCurrentTimeDilation) (Variables|TimeFX|GetTimeDilationStep))))

(event Custom|OnResetTime
  ;[1 1 1] Global time dilation
  (CallFunction|OnSetTimeDilation 1.0))

(event EventTick
  (params (DeltaSeconds :type Float%20%28single-precision%29)))

(fn ConstructionScript)