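; Game mode for a two-player lightsaber duel that spawns the combatants and routes hit damage.
; PostLogin spawns the first two players at PlayerStart transforms, pairs them as enemies, then initializes sabers and optional practice bot; later joiners become spectators.
; ApplyDamage applies point damage through a stub calculation returning a default value.
; Test events respawn the bot, toggle montage root motion with matching attack radius, and cycle server/client hit detection.
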(event Custom|ApplyDamage
  (params (hitResult :type Hit%20Result%20Structure) (CausedBy :type MCS%20Character%20Object%20Reference))
  ;[1 0.38 0.38] Calculate damage amount based on the hit information and game mode rules.
  (bind _output_get (Variables|Damage|SethitResult hitResult))
  (bind _damage (Damage|CalculateDamage _output_get))
  (Game|Damage|ApplyPointDamage (.HitActor (Collision|BreakHitResult _output_get)) _damage (.ImpactNormal (Collision|BreakHitResult _output_get)) (Variables|Damage|GethitResult) 0 CausedBy "/Script/Engine.DamageType"))

(event Custom|OnToggleRootMotion
  (bind _player_2 (Variables|CombatPlayers|GetPlayer_2))
  (bind _player_1 (Variables|CombatPlayers|GetPlayer_1))
  ;[0.495 1 0.7074] Server Options
  (bind _output_get (Variables|Options|SetUseRootMotion (not (Variables|Options|GetUseRootMotion))))
  (if _output_get
    (bind _asmcsanimation (Utilities|GetPlayerAnimInstance (Variables|CombatPlayers|GetPlayer_1)))
    (Class|AnimInstance|SetRootMotionMode _asmcsanimation "RootMotionFromMontagesOnly")
    (bind _asmcsanimation_2 (Utilities|GetPlayerAnimInstance (Variables|CombatPlayers|GetPlayer_2)))
    (Class|AnimInstance|SetRootMotionMode _asmcsanimation_2 "RootMotionFromMontagesOnly")
    (Variables|/Game/MCS/Blueprints/MCSCharacter.MCSCharacter_C|SetAttackRadius _player_1 (Variables|/Game/MCS/Blueprints/MCSCharacter.MCSCharacter_C|GetDefaultAttackRadius _player_1))
    (Variables|/Game/MCS/Blueprints/MCSCharacter.MCSCharacter_C|SetAttackRadius _player_2 (Variables|/Game/MCS/Blueprints/MCSCharacter.MCSCharacter_C|GetDefaultAttackRadius _player_2))
    (else
      (bind _asmcsanimation_3 (Utilities|GetPlayerAnimInstance (Variables|CombatPlayers|GetPlayer_1)))
      (Class|AnimInstance|SetRootMotionMode _asmcsanimation_3 "IgnoreRootMotion")
      (bind _asmcsanimation_4 (Utilities|GetPlayerAnimInstance (Variables|CombatPlayers|GetPlayer_2)))
      (Class|AnimInstance|SetRootMotionMode _asmcsanimation_4 "IgnoreRootMotion")
      (Variables|/Game/MCS/Blueprints/MCSCharacter.MCSCharacter_C|SetAttackRadius (Variables|CombatPlayers|GetPlayer_1) 8e+01)
      (Variables|/Game/MCS/Blueprints/MCSCharacter.MCSCharacter_C|SetAttackRadius (Variables|CombatPlayers|GetPlayer_2) 8e+01)))
  (if (Variables|Options|GetUseRootMotion)
    (Development|PrintString "Root Motion: ON")
    (else
      (Development|PrintString "Root Motion: OFF"))))

(event Custom|InitCombatPlayers
  ;[1 1 1] Initialize the combat players. Most of these values will come from the player selects in a "lobby".  i.e. Saber color, etc.
  (Utilities|FlowControl|Sequence
    (:then_0
      ;;[1 1 1] Hide players untill ready
      (Rendering|SetActorHiddenInGame (Variables|CombatPlayers|GetPlayer_1) false)
      (Rendering|SetActorHiddenInGame (Variables|CombatPlayers|GetPlayer_2) false))
    (:then_1
      ;;[1 1 1] Combat player 1
      (Default|ChangeSaberColor (Variables|CombatPlayers|GetPlayer_1) (Variables|CombatPlayers|GetPlayer1SaberColor))
      (bind _weapon (Utilities|GetPlayerWeapon (Variables|CombatPlayers|GetPlayer_1)))
      (Variables|/Game/MCS/Blueprints/Lightsaber.Lightsaber_C|SetHitDetectionType _weapon (Variables|Options|GetHitDetectionType))
      (Variables|/Game/MCS/Blueprints/Lightsaber.Lightsaber_C|SetNoCollisionWhenIdle _weapon (Variables|Options|GetNoCollisionWhenIdle)))
    (:then_2
      ;;[1 1 1] Combat Player 2
      (Default|ChangeSaberColor (Variables|CombatPlayers|GetPlayer_2) (Variables|CombatPlayers|GetPlayer2SaberColor))
      (bind _weapon_2 (Utilities|GetPlayerWeapon (Variables|CombatPlayers|GetPlayer_2)))
      (Variables|/Game/MCS/Blueprints/Lightsaber.Lightsaber_C|SetHitDetectionType _weapon_2 (Variables|Options|GetHitDetectionType))
      (Variables|/Game/MCS/Blueprints/Lightsaber.Lightsaber_C|SetNoCollisionWhenIdle _weapon_2 (Variables|Options|GetNoCollisionWhenIdle))
      (Variables|/Game/MCS/Blueprints/MCSCharacter.MCSCharacter_C|SetIsPracticeBot? (Variables|CombatPlayers|GetPlayer_2) (Variables|Options|GetbUseBot)))
    (:then_3
      ;;[1 1 1] Notify clients that the server is ready
      (Default|ServerIsReady (Variables|CombatPlayers|GetPlayer_1))
      (Default|ServerIsReady (Variables|CombatPlayers|GetPlayer_2)))))

(event Custom|CycleHitDetectionType
  ;[1 1 1] Cycle hit detection implementation for both combat players
  (switch Utilities|FlowControl|Switch|SwitchonMCSHitDetectionType (Variables|Options|GetHitDetectionType)
    (:NewEnumerator0
      (Variables|Options|SetHitDetectionType "NewEnumerator1"))
    (:NewEnumerator1
      (Variables|Options|SetHitDetectionType "NewEnumerator2"))
    (:NewEnumerator2
      (Variables|Options|SetHitDetectionType "NewEnumerator0")))
  (bind _weapon (Utilities|GetPlayerWeapon (Variables|CombatPlayers|GetPlayer_1)))
  (Variables|/Game/MCS/Blueprints/Lightsaber.Lightsaber_C|SetHitDetectionType _weapon (Variables|Options|GetHitDetectionType))
  (bind _weapon_2 (Utilities|GetPlayerWeapon (Variables|CombatPlayers|GetPlayer_2)))
  (Variables|/Game/MCS/Blueprints/Lightsaber.Lightsaber_C|SetHitDetectionType _weapon_2 (Variables|Options|GetHitDetectionType))
  (Development|PrintString (Utilities|String|Append "Hit Detection changed to: " (Utilities|String|EnumtoString (Variables|Options|GetHitDetectionType)))))

(event Custom|RespawnBot
  (bind _player_1 (Variables|CombatPlayers|GetPlayer_1))
  ;[1 1 1] FOR TESTING: Reset/Respawn the practice bot player
  (Actor|DestroyActor (Variables|CombatPlayers|GetPlayer_2))
  (Utilities|FlowControl|Delay 0.2)
  (bind _returnvalue (Game|SpawnActorfromClass "/Game/MCS/Blueprints/MCSCharacter.MCSCharacter_C" (Variables|CombatPlayers|GetPlayer2Transform) "Undefined" (Utilities|Array|Get(acopy) (Variables|Players|GetCurrentPlayers) 1) 0))
  (bind _output_get (Variables|CombatPlayers|SetPlayer_2 _returnvalue))
  (Pawn|Possess (Utilities|Array|Get(acopy) (Variables|Players|GetCurrentPlayers) 1) _output_get)
  (Utilities|FlowControl|Delay 1.0)
  (Default|OnSetEnemyPlayer (Variables|CombatPlayers|GetPlayer_2) (Variables|CombatPlayers|GetPlayer_2) (Variables|CombatPlayers|GetPlayer_1))
  (Default|OnSetEnemyPlayer _player_1 _player_1 (Variables|CombatPlayers|GetPlayer_2))
  (Default|ChangeSaberColor (Variables|CombatPlayers|GetPlayer_2) (Variables|CombatPlayers|GetPlayer2SaberColor))
  (Variables|/Game/MCS/Blueprints/MCSCharacter.MCSCharacter_C|SetIsPracticeBot? (Variables|CombatPlayers|GetPlayer_2) (Variables|Options|GetbUseBot))
  (Variables|/Game/MCS/Blueprints/MCSCharacter.MCSCharacter_C|SetHealth (Variables|CombatPlayers|GetPlayer_2) 1e+02)
  (Default|ServerIsReady (Variables|CombatPlayers|GetPlayer_2)))

(event EventPostLogin
  (params (NewPlayer :type Player%20Controller%20Object%20Reference))
  (bind _player_1 (Variables|CombatPlayers|GetPlayer_1))
  (bind _player_2 (Variables|CombatPlayers|GetPlayer_2))
  ;[1 1 1] Spawn combat player
  (Variables|Players|SetNewController NewPlayer)
  (if (< (Utilities|Array|Length (Variables|Players|GetCurrentPlayers)) 2)
    (PlayerSpawn|SpawnCombatPlayer (Variables|Players|GetNewController)) ; Once a player is spawned, he will be added to the currentPlayers array
    (if (== (Utilities|Array|Length (Variables|Players|GetCurrentPlayers)) 2) ; Do we have exactly 2 combat players
      (Utilities|FlowControl|Delay 1.0)
      (Default|OnSetEnemyPlayer _player_1 _player_1 (Variables|CombatPlayers|GetPlayer_2))
      (Default|OnSetEnemyPlayer _player_2 _player_2 (Variables|CombatPlayers|GetPlayer_1))
      (Utilities|FlowControl|Delay 1.0)
      (CallFunction|InitCombatPlayers))
    (else
      ;[1 1 1] Two combat players already spawned.  Spawn spectator(s)
      (bind _returnvalue (Game|SpawnActorfromClass "/Game/MCS/Blueprints/MCSSpectatorPawn.MCSSpectatorPawn_C" (Math|Transform|MakeTransform (Variables|Spectator|GetSpectatorStartLocation)) "Undefined" 0 0))
      (bind _output_get (Variables|Spectator|SetNewSpectator _returnvalue))
      (Pawn|Possess (Variables|Players|GetNewController) _output_get))))

(event EventHandleStartingNewPlayer
  (params (NewPlayer :type Player%20Controller%20Object%20Reference)))

(event EventBeginPlay
  ;[1 1 1] Initialize spawn locations for combat players
  (PlayerSpawn|SetSpawnLocations))

(fn ConstructionScript)

(fn CalculateDamage
  (params (hitResult :type Hit%20Result%20Structure))
  ;[1 1 1] STUB: Calculate damage here
  (return (Variables|Damage|GetDefaultBaseDamage)))

(fn SetSpawnLocations
  (bind _outactors (Actor|GetAllActorsOfClass "/Script/Engine.PlayerStart"))
  (bind _output_get (Variables|Players|SetPlayerStartArray _outactors))
  (if (> (Utilities|Array|Length _output_get) 0) ; We have at least 1 player start actor
    (bind (_array_element _array_index) (Utilities|Array|ForEachLoopwithBreak (Variables|Players|GetPlayerStartArray) :!label _label)
      (:LoopBody
        (LocalVariables|SetcurrentPlayerStart _array_element)
        (bind _output_get_2 (LocalVariables|SetcurrentIndex _array_index))
        (if (<= _output_get_2 1) ; If more than 2 player start actors, then exit
          (if (== (LocalVariables|GetcurrentIndex) 0) ; First player start
            (Variables|CombatPlayers|SetPlayer1Transform (Transformation|GetActorTransform (LocalVariables|GetcurrentPlayerStart)))
            (elif (== (LocalVariables|GetcurrentIndex) 1) ; Second player start
              (Variables|CombatPlayers|SetPlayer2Transform (Transformation|GetActorTransform (LocalVariables|GetcurrentPlayerStart)))))
          (else
            (goto _label Break)))))))

(fn SpawnCombatPlayer
  (params (Player :type Player%20Controller%20Object%20Reference))
  (LocalVariables|SetcombatPlayer Player)
  (if (< (Utilities|Array|Length (Variables|Players|GetCurrentPlayers)) 1)
    (bind _returnvalue (Game|SpawnActorfromClass "/Game/MCS/Blueprints/MCSCharacter.MCSCharacter_C" (Variables|CombatPlayers|GetPlayer1Transform) "Undefined" (LocalVariables|GetcombatPlayer) 0))
    (bind _output_get (Variables|CombatPlayers|SetPlayer_1 _returnvalue))
    (Pawn|Possess (LocalVariables|GetcombatPlayer) _output_get)
    (Utilities|Array|Add (Variables|Players|GetCurrentPlayers) (LocalVariables|GetcombatPlayer))
    (else
      (bind _returnvalue_2 (Game|SpawnActorfromClass "/Game/MCS/Blueprints/MCSCharacter.MCSCharacter_C" (Variables|CombatPlayers|GetPlayer2Transform) "Undefined" (LocalVariables|GetcombatPlayer) 0))
      (bind _output_get_2 (Variables|CombatPlayers|SetPlayer_2 _returnvalue_2))
      (Pawn|Possess (LocalVariables|GetcombatPlayer) _output_get_2)
      (Utilities|Array|Add (Variables|Players|GetCurrentPlayers) (LocalVariables|GetcombatPlayer)))))