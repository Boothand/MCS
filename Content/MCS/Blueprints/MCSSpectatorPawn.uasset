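; Spectator pawn for MCS that can follow and look at the player's character.
; While LookAtPlayer is set, each Tick finds the first MCSCharacter and snaps the pawn to a fixed horizontal offset from it at a constant height.
; It then turns its controller's rotation toward that character, giving an elevated tracking camera view.
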(event EventBeginPlay)

(event Collision|EventActorBeginOverlap
  (params (OtherActor :type Actor%20Object%20Reference)))

(event EventTick
  (params (DeltaSeconds :type Float%20%28single-precision%29))
  (bind _returnvalue (Pawn|GetController))
  (if (Variables|Default|GetbLookAtPlayer)
    (bind _outactors (Actor|GetAllActorsOfClass "/Game/MCS/Blueprints/MCSCharacter.MCSCharacter_C"))
    (Utilities|IsValid (Utilities|Array|Get(acopy) _outactors)
      (:Is%20Valid
        (Utilities|IsValid _returnvalue
          (:Is%20Valid
            (Transformation|SetActorLocation (Math|Vector|MakeVector (+ (.X (Math|Vector|BreakVector (Transformation|GetActorLocation (Utilities|Array|Get(acopy) _outactors)))) 3e+02) (- (.Y (Math|Vector|BreakVector (Transformation|GetActorLocation (Utilities|Array|Get(acopy) _outactors)))) 4e+02) 6e+02) false false)
            (Pawn|SetControlRotation _returnvalue (Math|Rotator|FindLookatRotation (Transformation|GetActorLocation) (Transformation|GetActorLocation (Utilities|Array|Get(acopy) _outactors))))))))))

(fn ConstructionScript)